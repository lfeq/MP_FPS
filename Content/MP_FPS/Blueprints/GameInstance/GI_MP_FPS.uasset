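; Game instance for the multiplayer FPS that centralizes menu display, game start and online session management.
; Events create and show the main, multiplayer and server list widgets, with the main menu switching to UI-only input.
; Single player opens First_Level directly, while hosting creates a non-LAN session and opens it as a listen server, both restoring game input.
; Join and destroy events wrap the session nodes, printing failures for host and join.
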(event Custom|ShowMltiplayerMenu
  (bind _returnvalue (UserInterface|CreateWidget "/Game/MP_FPS/Blueprints/Widgets/UI/BPW_MultiplayerMenu.BPW_MultiplayerMenu_C" (Game|GetPlayerController 0)))
  (bind _output_get (Variables|Default|SetmultiplayerMenuReference _returnvalue))
  (UserInterface|Viewport|AddtoViewport _output_get 0))

(event Custom|JoinSession
  (params (session :type Blueprint%20Session%20Result%20Structure))
  (|JoinSession (Game|GetPlayerController 0) session
    (:OnFailure
      (Development|PrintString "Failed to join session"))))

(event Custom|ShowServerList
  (bind _returnvalue (UserInterface|CreateWidget "/Game/MP_FPS/Blueprints/Widgets/UI/BPW_ServerList.BPW_ServerList_C" (Game|GetPlayerController 0)))
  (bind _output_get (Variables|Default|SetserverListReference _returnvalue))
  (UserInterface|Viewport|AddtoViewport _output_get 0))

(event Custom|StartSinglePlayer
  (bind _returnvalue (Game|GetPlayerController 0))
  (Game|OpenLevel(byName) "First_Level")
  (Input|SetInputModeGameOnly _returnvalue)
  (Variables|/Script/Engine.PlayerController|SetbShowMouseCursor _returnvalue false))

(event Custom|DestroySessionCaller
  (params (playerController :type Player%20Controller%20Object%20Reference))
  (|DestroySession playerController))

(event Custom|HostGame
  (bind _returnvalue (Game|GetPlayerController 0))
  (|Session _returnvalue 10 false
    (:OnSuccess
      (Game|OpenLevel(byName) "First_Level" true "listen")
      (Input|SetInputModeGameOnly _returnvalue)
      (Variables|/Script/Engine.PlayerController|SetbShowMouseCursor _returnvalue false))
    (:OnFailure
      (Development|PrintString "Host game failed"))))

(event Custom|ShowMainMenu
  (bind _returnvalue (Game|GetPlayerController 0))
  (bind _returnvalue_2 (UserInterface|CreateWidget "/Game/MP_FPS/Blueprints/Widgets/UI/BPW_MainMenu.BPW_MainMenu_C" _returnvalue))
  (bind _output_get (Variables|Default|SetmainMenuReference _returnvalue_2))
  (UserInterface|Viewport|AddtoViewport _output_get 0)
  (Input|SetInputModeUIOnly _returnvalue _output_get "DoNotLock")
  (Variables|/Script/Engine.PlayerController|SetbShowMouseCursor _returnvalue true))