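; Base multiplayer FPS character with team colors, an overhead name and health tag, weapons, sprinting and grenade throwing.
; The server spawns a two-weapon loadout, gates fire, sprint and weapon toggle through Can checks, and multicasts weapon swaps between hand and holster sockets.
; Damage from other teams' players lowers replicated health; death multicasts a ragdoll, then requests a timed respawn.
; OnRep functions update the tag widget and team-colored dynamic materials.
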(event Custom|ServerStartSprint
  ;[1 1 1] Set sprint
  (bind _cansprint (CallFunction|CanSprint))
  (if _cansprint
    (Variables|Default|SetisSprinting true)
    (Variables|/Script/Engine.CharacterMovementComponent|SetMaxWalkSpeed (Variables|Character|GetCharacterMovement) 6e+02)
    (CallFunction|ClientStartSprint)
    (Variables|/Script/Engine.CharacterMovementComponent|SetMaxWalkSpeed (Variables|Character|GetCharacterMovement) 6e+02)))

(event Custom|ClientStopSprint
  (Variables|/Script/Engine.CharacterMovementComponent|SetMaxWalkSpeed (Variables|Character|GetCharacterMovement) 1.8e+02))

(event Custom|MulticastToggleWeapon
  (Utilities|FlowControl|Sequence
    (:then_0
      ;[1 1 1] Toggle weapon logic
      (if (> (+ (Variables|Default|GetweaponIndex) 1) (- (Utilities|Array|Length (Variables|Default|GetweaponInventoryReference)) 1))
        (Variables|Default|SetweaponIndex 0)
        (else
          (Variables|Default|SetweaponIndex (+ (Variables|Default|GetweaponIndex) 1)))))
    (:then_1
      ;[1 1 1] Toggle weapon meshes
      (Utilities|FlowControl|Delay 0.4)
      (Transformation|AttachComponentToComponent (Variables|Default|GetCurrentWeaponReference) (Variables|Character|GetMesh) (Variables|Default|GetholsterSocketName) "SnapToTarget" "SnapToTarget" "KeepWorld" true)
      (Transformation|AttachComponentToComponent (Variables|/Game/MP_FPS/Blueprints/Weapons/BP_WeaponMaster.BP_WeaponMaster_C|GetSK_FP_Weapon (Variables|Default|GetCurrentWeaponReference)) (Variables|Character|GetMesh) (Variables|Default|GetholsterSocketName) "SnapToTarget" "SnapToTarget" "KeepWorld" true)
      (Transformation|AttachComponentToComponent (Variables|/Game/MP_FPS/Blueprints/Weapons/BP_WeaponMaster.BP_WeaponMaster_C|GetSK_TP_Weapon (Variables|Default|GetCurrentWeaponReference)) (Variables|Character|GetMesh) (Variables|Default|GetholsterSocketName) "SnapToTarget" "SnapToTarget" "KeepWorld" true)
      (Utilities|FlowControl|Sequence
        (:then_0
          (CallFunction|MulticasSetShadow1))
        (:then_1
          (Rendering|SetActorHiddenInGame (Variables|Default|GetCurrentWeaponReference) true)
          (Transformation|AttachComponentToComponent (Utilities|Array|Get(acopy) (Variables|Default|GetweaponInventoryReference) (Variables|Default|GetweaponIndex)) (Variables|Default|GetSK_Arms) (Variables|/Game/MP_FPS/Blueprints/Weapons/BP_WeaponMaster.BP_WeaponMaster_C|GetweaponSocketName (Utilities|Array|Get(acopy) (Variables|Default|GetweaponInventoryReference) (Variables|Default|GetweaponIndex))) "SnapToTarget" "SnapToTarget" "KeepWorld" true)
          (Variables|Default|SetCurrentWeaponReference (Utilities|Array|Get(acopy) (Variables|Default|GetweaponInventoryReference) (Variables|Default|GetweaponIndex)))
          (Transformation|AttachComponentToComponent (Variables|/Game/MP_FPS/Blueprints/Weapons/BP_WeaponMaster.BP_WeaponMaster_C|GetSK_FP_Weapon (Utilities|Array|Get(acopy) (Variables|Default|GetweaponInventoryReference) (Variables|Default|GetweaponIndex))) (Variables|Default|GetSK_Arms) (Variables|/Game/MP_FPS/Blueprints/Weapons/BP_WeaponMaster.BP_WeaponMaster_C|GetweaponSocketName (Utilities|Array|Get(acopy) (Variables|Default|GetweaponInventoryReference) (Variables|Default|GetweaponIndex))) "SnapToTarget" "SnapToTarget" "KeepWorld" true)
          (Transformation|AttachComponentToComponent (Variables|/Game/MP_FPS/Blueprints/Weapons/BP_WeaponMaster.BP_WeaponMaster_C|GetSK_TP_Weapon (Utilities|Array|Get(acopy) (Variables|Default|GetweaponInventoryReference) (Variables|Default|GetweaponIndex))) (Variables|Character|GetMesh) (Variables|/Game/MP_FPS/Blueprints/Weapons/BP_WeaponMaster.BP_WeaponMaster_C|GetweaponSocketName (Utilities|Array|Get(acopy) (Variables|Default|GetweaponInventoryReference) (Variables|Default|GetweaponIndex))) "SnapToTarget" "SnapToTarget" "KeepWorld" true)
          (Utilities|FlowControl|Sequence
            (:then_0
              (CallFunction|ServerSetShadow2))
            (:then_1
              (Rendering|SetActorHiddenInGame (Variables|Default|GetCurrentWeaponReference) false))))))))

(event Custom|ServerThrowGrenade
  (bind _fp_camera (Variables|Default|GetFP_Camera))
  (bind _returnvalue (Transformation|GetWorldRotation _fp_camera))
  (bind _returnvalue_2 (Game|SpawnActorfromClass "/Game/MP_FPS/Blueprints/Weapons/BP_Grenade.BP_Grenade_C" (Math|Transform|MakeTransform (Transformation|GetWorldLocation (Variables|Default|GetFP_Camera)) _returnvalue "1,1,1") "AdjustIfPossibleButAlwaysSpawn" (Components|GetOwner) (Game|GetInstigator)))
  (Physics|SetPhysicsLinearVelocity (Variables|/Game/MP_FPS/Blueprints/Weapons/BP_Grenade.BP_Grenade_C|GetSM_Grenade _returnvalue_2) (* (Math|Vector|GetForwardVector _returnvalue) 1e+03) false "None"))

(event Custom|MulticastRagdoll
  ;[1 1 1] Activate Ragdoll
  (CallFunction|Ragdoll))

(event Custom|ServerStartWeaponFire
  (bind _currentweaponreference (Variables|Default|GetCurrentWeaponReference))
  (bind _canfire (CallFunction|CanFire))
  (if _canfire
    (Variables|/Game/MP_FPS/Blueprints/Weapons/BP_WeaponMaster.BP_WeaponMaster_C|SetisCooldownActive _currentweaponreference true)
    (Variables|Default|SetisFiringWeapon true)
    (Default|ClientonWeaponFire _currentweaponreference)))

(event Custom|ServerToggleWeapon
  (bind _cantoggle (CallFunction|CanToggleWeapon))
  (if _cantoggle
    (Variables|Default|SetisTogglingWeapon true)
    (CallFunction|MulticastToggleWeapon)))

(event Custom|ServerDestroyCharacter
  (bind _currentweaponreference (Variables|Default|GetCurrentWeaponReference))
  (Utilities|IsValid _currentweaponreference
    (:Is%20Valid
      (Actor|DestroyActor _currentweaponreference))
    (:Is%20Not%20Valid
      _))
  (Actor|DestroyActor))

(event Custom|ClientThrowGrenade
  (CallFunction|ServerThrowGrenade))

(event Custom|ServerStopSprint
  ;[1 1 1] Set sprint
  (Variables|Default|SetisSprinting false)
  (Variables|/Script/Engine.CharacterMovementComponent|SetMaxWalkSpeed (Variables|Character|GetCharacterMovement) 1.8e+02)
  (CallFunction|ClientStopSprint)
  (Variables|/Script/Engine.CharacterMovementComponent|SetMaxWalkSpeed (Variables|Character|GetCharacterMovement) 1.8e+02))

(event Custom|ServerStopWeaponFire
  (Variables|Default|SetisFiringWeapon false)
  (Default|ClientOffWeaponFire (Variables|Default|GetCurrentWeaponReference)))

(event Custom|MulticasSetShadow1
  (bind _currentweaponreference (Variables|Default|GetCurrentWeaponReference))
  (Rendering|SetCastShadow (Variables|/Game/MP_FPS/Blueprints/Weapons/BP_WeaponMaster.BP_WeaponMaster_C|GetSK_FP_Weapon _currentweaponreference) false)
  (Rendering|SetCastShadow (Variables|/Game/MP_FPS/Blueprints/Weapons/BP_WeaponMaster.BP_WeaponMaster_C|GetSK_TP_Weapon _currentweaponreference) false))

(event Custom|ClientRespawn
  (bind _aspc_mp_fps (Utilities|Casting|CastToPC_MP_FPS (Game|GetPlayerController 0)))
  (Default|ServerRequestRespawn _aspc_mp_fps))

(event Custom|ServerSetShadow2
  (Rendering|SetCastShadow (Variables|/Game/MP_FPS/Blueprints/Weapons/BP_WeaponMaster.BP_WeaponMaster_C|GetSK_TP_Weapon (Variables|Default|GetCurrentWeaponReference)) false)
  (CallFunction|MulticastSetShadow2))

(event Custom|ClientStartSprint
  (Variables|/Script/Engine.CharacterMovementComponent|SetMaxWalkSpeed (Variables|Character|GetCharacterMovement) 6e+02))

(event Custom|ServerKillPlayerNoRagdoll
  (CallFunction|ClientRespawn))

(event Custom|MulticastSetShadow2
  (Rendering|SetCastShadow (Variables|/Game/MP_FPS/Blueprints/Weapons/BP_WeaponMaster.BP_WeaponMaster_C|GetSK_TP_Weapon (Variables|Default|GetCurrentWeaponReference)) true))

(event Custom|MulticastSetShadow
  ;[1 1 1] Toggle shadows on begin play
  (Rendering|SetCastShadow (Variables|/Game/MP_FPS/Blueprints/Weapons/BP_WeaponMaster.BP_WeaponMaster_C|GetSK_TP_Weapon (Variables|Default|GetsecondaryWeaponReference)) false))

(event Custom|ServerKillPlayer
  (Utilities|FlowControl|DoOnce false
    (:Completed
      (Variables|Default|SetisDead true)
      (Variables|Default|SetcurrentHealth 0)
      (CallFunction|MulticastRagdoll)
      (if (not (AI|Components|NavMovement|IsFalling (Variables|Character|GetCharacterMovement)))
        (Utilities|FlowControl|Delay (Variables|Default|GetrespawnTimer))
        (CallFunction|ClientRespawn)))))

(event EventBeginPlay
  (Utilities|FlowControl|Sequence
    (:then_0
      ;[1 1 1] Setup weapon
      (Networking|SwitchHasAuthority
        (:Authority
          (CallFunction|GiveDefaultLoadout)
          (Utilities|FlowControl|Delay 0.5)
          (CallFunction|MulticastSetShadow))))
    (:then_1
      ;[1 1 1] Initialize Health
      (Networking|SwitchHasAuthority
        (:Authority
          (Variables|Default|SetcurrentHealth (Variables|Default|GetmaxHealth)))
        (:Remote
          (CallFunction|ClientUpdateHealth))))
    (:then_2
      ;[1 1 1] Set Player name over player
      (Networking|SwitchHasAuthority
        (:Authority
          (Utilities|FlowControl|Delay 0.5)
          (bind _asps_ms_fps (Utilities|Casting|CastToPS_MS_FPS (Variables|GetPlayerState)))
          (Variables|Default|SetlocalPlayerName (Variables|/Game/MP_FPS/Blueprints/Characters/PS_MS_FPS.PS_MS_FPS_C|GetplayerSetName _asps_ms_fps)))
        (:Remote
          (CallFunction|ClientUpdatePlayerName))))))

(event Game|Damage|EventAnyDamage
  (params (Damage :type Float%20%28single-precision%29) (DamageType :type Damage%20Type%20Object%20Reference) (InstigatedBy :type Controller%20Object%20Reference) (DamageCauser :type Actor%20Object%20Reference))
  ;[1 1 1] Event Any Damage
  (bind _aspc_mp_fps (Utilities|Casting|CastToPC_MP_FPS InstigatedBy))
  (if (not (Utilities|Enum|Equal(Enum) (Variables|/Game/MP_FPS/Blueprints/Characters/PC_MP_FPS.PC_MP_FPS_C|Getteam _aspc_mp_fps) (Variables|Default|Getteam)))
    (bind _output_get (Variables|Default|SetcurrentHealth (Math|Integer|Clamp(Integer) (Math|Float|Truncate (- (Math|Conversions|ToFloat(Integer) (Variables|Default|GetcurrentHealth)) Damage)) 0 (Variables|Default|GetmaxHealth))))
    (if (<= _output_get 0)
      (CallFunction|ServerKillPlayer))))

(event EventOnLanded
  (params (Hit :type Hit%20Result%20Structure%20%28by%20ref%29))
  (Networking|SwitchHasAuthority
    (:Authority
      (if (Variables|Default|GetisDead)
        (Utilities|FlowControl|Delay (Variables|Default|GetrespawnTimer))
        (CallFunction|ClientRespawn)))))

(event EventUnpossessed
  (params (OldController :type Controller%20Object%20Reference))
  (Networking|SwitchHasAuthority
    (:Authority
      (CallFunction|ServerDestroyCharacter))))

(event Input|ActionEvents|InputActionJump
  (params (Key :type Key%20Structure :default "AnyKey"))
  (bind _isdead (Variables|Default|GetisDead))
  (bind _returnvalue (not _isdead))
  ;[1 1 1] Handle jump
  (:Pressed
    (if _returnvalue
      (Character|Jump)))
  (:Released
    (if _returnvalue
      (Character|StopJumping))))

(event Input|ActionEvents|InputActionFireWeapon
  (params (Key :type Key%20Structure :default "AnyKey"))
  ;[1 1 1] Fire weapon input
  (:Pressed
    (CallFunction|ServerStartWeaponFire))
  (:Released
    (CallFunction|ServerStopWeaponFire)))

(event Input|ActionEvents|InputActionToggleWeapon
  (params (Key :type Key%20Structure :default "AnyKey"))
  (:Pressed
    (CallFunction|ServerToggleWeapon)))

(event Input|ActionEvents|InputActionForceRespawn
  (params (Key :type Key%20Structure :default "AnyKey"))
  (:Pressed
    (CallFunction|ServerKillPlayer)))

(event Input|ActionEvents|InputActionSprint
  (params (Key :type Key%20Structure :default "AnyKey"))
  ;[1 1 1] Handle Sprint
  (:Pressed
    (CallFunction|ServerStartSprint))
  (:Released
    (CallFunction|ServerStopSprint)))

(event Input|AxisEvents|InputAxisMoveForward
  (params (AxisValue :type Float%20%28single-precision%29))
  ;[1 1 1] Handle movement input
  (if (not (Variables|Default|GetisDead))
    (Pawn|Input|AddMovementInput (Math|Vector|GetForwardVector (Math|Rotator|MakeRotator 0.0 0.0 (.yaw (Pawn|GetControlRotation :!class /Script/Engine.Pawn)))) AxisValue false)
    (if (Variables|Default|GetisSprinting)
      (if (<= AxisValue 0.0)
        (CallFunction|ServerStopSprint)))))

(event Input|AxisEvents|InputAxisLookUp
  (params (AxisValue :type Float%20%28single-precision%29))
  ;[1 1 1] Handle Mouse Camera Movement
  (Pawn|Input|AddControllerPitchInput AxisValue))

(event Input|AxisEvents|InputAxisTurn
  (params (AxisValue :type Float%20%28single-precision%29))
  ;[1 1 1] Handle Mouse Camera Movement
  (Pawn|Input|AddControllerYawInput AxisValue))

(event Input|AxisEvents|InputAxisMoveRight
  (params (AxisValue :type Float%20%28single-precision%29))
  ;[1 1 1] Handle movement input
  (if (not (Variables|Default|GetisDead))
    (Pawn|Input|AddMovementInput (Math|Vector|GetRightVector (Math|Rotator|MakeRotator 0.0 0.0 (.yaw (Pawn|GetControlRotation :!class /Script/Engine.Pawn)))) AxisValue false)))

(event Input|KeyboardEvents|G
  (params (Key :type Key%20Structure :default "AnyKey"))
  (:Pressed
    (CallFunction|ClientThrowGrenade)))

(fn ConstructionScript
  (bind _returnvalue (Rendering|Material|CreateDynamicMaterialInstance (Variables|Character|GetMesh) 0 "/Game/MP_FPS/Materials/M_TeamColor.M_TeamColor" :!class /Script/Engine.PrimitiveComponent))
  (Variables|Default|SetbodyDynamicMaterial _returnvalue)
  (bind _returnvalue_2 (Rendering|Material|CreateDynamicMaterialInstance (Variables|Default|GetSK_Arms) 0 "/Game/MP_FPS/Materials/M_TeamColor.M_TeamColor" :!class /Script/Engine.PrimitiveComponent))
  (Variables|Default|SetarmsDynamicMaterial _returnvalue_2)
  (bind _returnvalue_3 (Rendering|Material|CreateDynamicMaterialInstance (Variables|Default|GetSK_Torso) 0 "/Game/MP_FPS/Materials/M_TeamColor.M_TeamColor" :!class /Script/Engine.PrimitiveComponent))
  (Variables|Default|SettorsoDynamicMaterial _returnvalue_3)
  (Rendering|Material|SetVectorParameterValue (Variables|Default|GetbodyDynamicMaterial) "Color" (Utilities|Select :Index (Variables|Default|Getteam) :NewEnumerator0 "(R=1.000000,G=0.000000,B=0.823312,A=1.000000)" :NewEnumerator1 "(R=1.000000,G=0.000000,B=0.129168,A=1.000000)" :NewEnumerator2 "(R=0.000000,G=0.115681,B=1.000000,A=1.000000)") :!class /Script/Engine.MaterialInstanceDynamic))

(fn OnRepCurrentHealth
  (bind _asbpw_player_tag (Utilities|Casting|CastToBPW_PlayerTag (UserInterface|GetUserWidgetObject (Variables|Default|GetBPW_PlayerTag))))
  (Progress|SetPercent (Variables|/Game/MP_FPS/Blueprints/Widgets/BPW_PlayerTag.BPW_PlayerTag_C|GetHealthbar _asbpw_player_tag) (/ (Math|Conversions|ToFloat(Integer) (Variables|Default|GetcurrentHealth)) (Math|Conversions|ToFloat(Integer) (Variables|Default|GetmaxHealth)))))

(fn OnRepLocalPlayerName
  (bind _asbpw_player_tag (Utilities|Casting|CastToBPW_PlayerTag (UserInterface|GetUserWidgetObject (Variables|Default|GetBPW_PlayerTag))))
  (Rendering|Components|TextRender|SetText (Variables|/Game/MP_FPS/Blueprints/Widgets/BPW_PlayerTag.BPW_PlayerTag_C|GetText_PlayerName _asbpw_player_tag) (Utilities|Text|ToText(String) (Variables|Default|GetlocalPlayerName))))

(fn ClientUpdateHealth
  (bind _asbpw_player_tag (Utilities|Casting|CastToBPW_PlayerTag (UserInterface|GetUserWidgetObject (Variables|Default|GetBPW_PlayerTag))))
  (Progress|SetPercent (Variables|/Game/MP_FPS/Blueprints/Widgets/BPW_PlayerTag.BPW_PlayerTag_C|GetHealthbar _asbpw_player_tag) (/ (Math|Conversions|ToFloat(Integer) (Variables|Default|GetcurrentHealth)) (Math|Conversions|ToFloat(Integer) (Variables|Default|GetmaxHealth)))))

(fn ClientUpdatePlayerName
  (bind _asbpw_player_tag (Utilities|Casting|CastToBPW_PlayerTag (UserInterface|GetUserWidgetObject (Variables|Default|GetBPW_PlayerTag))))
  (Rendering|Components|TextRender|SetText (Variables|/Game/MP_FPS/Blueprints/Widgets/BPW_PlayerTag.BPW_PlayerTag_C|GetText_PlayerName _asbpw_player_tag) (Utilities|Text|ToText(String) (Variables|Default|GetlocalPlayerName))))

(fn GiveDefaultLoadout
  (bind _self self)
  (bind _self_2 self)
  (bind _weaponsocketname (Variables|Default|GetweaponSocketName))
  (bind _weaponinventoryreference (Variables|Default|GetweaponInventoryReference))
  (bind _sk_arms (Variables|Default|GetSK_Arms))
  (bind _item (Utilities|Array|Get(acopy) _weaponinventoryreference 1))
  (bind _returnvalue (Transformation|GetSocketTransform _sk_arms _weaponsocketname "RTS_World"))
  (Utilities|FlowControl|Sequence
    (:then_0
      ;[1 1 1] Spawn weapons
      (bind _returnvalue_2 (Game|SpawnActorfromClass (Variables|Default|GetprimaryWeapon) _returnvalue "AlwaysSpawn" _self _self _self))
      (Variables|Default|SetprimaryWeaponReference _returnvalue_2)
      (Utilities|Array|Add (Variables|Default|GetweaponInventoryReference) _returnvalue_2)
      (bind _returnvalue_3 (Game|SpawnActorfromClass (Variables|Default|GetsecondaryWeapon) _returnvalue "AlwaysSpawn" _self_2 _self_2 _self_2))
      (Variables|Default|SetsecondaryWeaponReference _returnvalue_3)
      (Utilities|Array|Add (Variables|Default|GetweaponInventoryReference) _returnvalue_3))
    (:then_1
      ;[1 1 1] Attach weapons to sockets
      (bind _output_get (Variables|Default|SetCurrentWeaponReference (Utilities|Array|Get(acopy) (Variables|Default|GetweaponInventoryReference))))
      (Transformation|AttachComponentToComponent _output_get (Variables|Character|GetMesh) (Variables|/Game/MP_FPS/Blueprints/Weapons/BP_WeaponMaster.BP_WeaponMaster_C|GetweaponSocketName _output_get) "SnapToTarget" "SnapToTarget" "KeepWorld" true)
      (Transformation|AttachComponentToComponent (Variables|/Game/MP_FPS/Blueprints/Weapons/BP_WeaponMaster.BP_WeaponMaster_C|GetSK_FP_Weapon (Variables|Default|GetCurrentWeaponReference)) (Variables|Default|GetSK_Arms) (Variables|/Game/MP_FPS/Blueprints/Weapons/BP_WeaponMaster.BP_WeaponMaster_C|GetweaponSocketName _output_get) "SnapToTarget" "SnapToTarget" "KeepWorld" true)
      (Transformation|AttachComponentToComponent (Variables|/Game/MP_FPS/Blueprints/Weapons/BP_WeaponMaster.BP_WeaponMaster_C|GetSK_TP_Weapon (Variables|Default|GetCurrentWeaponReference)) (Variables|Character|GetMesh) (Variables|/Game/MP_FPS/Blueprints/Weapons/BP_WeaponMaster.BP_WeaponMaster_C|GetweaponSocketName _output_get) "SnapToTarget" "SnapToTarget" "KeepWorld" true)
      (Transformation|AttachComponentToComponent _item (Variables|Character|GetMesh) (Variables|Default|GetholsterSocketName) "SnapToTarget" "SnapToTarget" "KeepWorld" true)
      (Rendering|SetActorHiddenInGame _item true)
      (Variables|Default|SetweaponIndex 0))))

(fn Ragdoll
  (bind _currentweaponreference (Variables|Default|GetCurrentWeaponReference))
  (bind _mesh (Variables|Character|GetMesh))
  (Development|SetHiddeninGame (Variables|/Game/MP_FPS/Blueprints/Weapons/BP_WeaponMaster.BP_WeaponMaster_C|GetSK_FP_Weapon _currentweaponreference) true false)
  (Class|PrimitiveComponent|SetOwnerNoSee (Variables|/Game/MP_FPS/Blueprints/Weapons/BP_WeaponMaster.BP_WeaponMaster_C|GetSK_TP_Weapon _currentweaponreference) false)
  (Physics|SetSimulatePhysics (Variables|Default|GetSK_Arms) true)
  (Collision|SetCollisionResponsetoChannel _mesh "ECC_Pawn" "ECR_Ignore")
  (Collision|SetCollisionEnabled _mesh "QueryAndPhysics")
  (Collision|SetCollisionResponsetoChannel (Variables|Collision|GetCapsuleComponent) "ECC_Pawn" "ECR_Ignore"))

(fn CanFire
  (bind _currentweaponreference (Variables|Default|GetCurrentWeaponReference))
  (Networking|SwitchHasAuthority
    (:Authority
      (Utilities|IsValid _currentweaponreference
        (:Is%20Valid
          (if (Math|Boolean|ANDBoolean (not (Variables|/Game/MP_FPS/Blueprints/Weapons/BP_WeaponMaster.BP_WeaponMaster_C|GetisCooldownActive _currentweaponreference)) (not (Variables|Default|GetisDead)) (not (Variables|Default|GetisFiringWeapon)) (not (Variables|Default|GetisTogglingWeapon)) (not (Variables|Default|GetisSprinting)))
            (Variables|Default|SetcanFire? true)
            (else
              (Variables|Default|SetcanFire? false))))
        (:Is%20Not%20Valid
          _))
      (return (Variables|Default|GetcanFire?)))))

(fn CanSprint
  (Networking|SwitchHasAuthority
    (:Authority
      (if (Math|Boolean|ANDBoolean (not (Variables|Default|GetisDead)) (not (Variables|Default|GetisFiringWeapon)) (not (Variables|Default|GetisTogglingWeapon)) (not (Variables|Default|GetisSprinting)))
        (Variables|Default|SetcanSprint? true)
        (else
          (Variables|Default|SetcanSprint? false :!label _label))))
    (:Remote
      (goto _label)))
  (return (Variables|Default|GetcanSprint?)))

(fn CanToggleWeapon
  (bind _currentweaponreference (Variables|Default|GetCurrentWeaponReference))
  (Networking|SwitchHasAuthority
    (:Authority
      (Utilities|IsValid _currentweaponreference
        (:Is%20Valid
          (if (Math|Boolean|ANDBoolean (not (Variables|/Game/MP_FPS/Blueprints/Weapons/BP_WeaponMaster.BP_WeaponMaster_C|GetisCooldownActive _currentweaponreference)) (not (Variables|Default|GetisDead)) (not (Variables|Default|GetisFiringWeapon)) (not (Variables|Default|GetisTogglingWeapon)) (not (Variables|Default|GetisSprinting)))
            (Variables|Default|SetcanToggleWeapon? true)
            (else
              (Variables|Default|SetcanToggleWeapon? false :!label _label))))
        (:Is%20Not%20Valid
          (goto _label))))
    (:Remote
      (goto _label)))
  (return (Variables|Default|GetcanToggleWeapon?)))

(fn OnRepTeam
  (Rendering|Material|SetVectorParameterValue (Variables|Default|GetbodyDynamicMaterial) "Color" (Utilities|Select :Index (Variables|Default|Getteam) :NewEnumerator0 "(R=1.000000,G=0.000000,B=0.823312,A=1.000000)" :NewEnumerator1 "(R=1.000000,G=0.000000,B=0.129168,A=1.000000)" :NewEnumerator2 "(R=0.000000,G=0.115681,B=1.000000,A=1.000000)") :!class /Script/Engine.MaterialInstanceDynamic))