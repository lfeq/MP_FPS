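; Game mode for the multiplayer FPS that manages team spawn points and respawns players.
; Shortly after BeginPlay, the server sorts all BP_TeamStartMaster actors into lobby, red and blue spawn point arrays by team.
; ServerRespawnPlayer spawns a BP_CharacterMaster with the requested team at a random point from that team's array, adjusting for collisions but always spawning, then has the player controller possess it.
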(event Custom|ServerRespawnPlayer
  (params (PlayerController :type Player%20Controller%20Object%20Reference) (team :type E_Teams%20Enum))
  (bind _lobbyspawnpoints (Variables|Default|GetlobbySpawnPoints))
  (bind _redteamspawnpoints (Variables|Default|GetredTeamSpawnPoints))
  (bind _blueteamspawnpoints (Variables|Default|GetblueTeamSpawnPoints))
  (bind _returnvalue (Utilities|Select :Index team :NewEnumerator0 _lobbyspawnpoints :NewEnumerator1 _redteamspawnpoints :NewEnumerator2 _blueteamspawnpoints))
  (bind _returnvalue_2 (Utilities|Array|Length _returnvalue))
  (bind _returnvalue_3 (- _returnvalue_2 1))
  (bind _returnvalue_4 (Math|Random|RandomIntegerinRange 0 _returnvalue_3))
  (bind _item (Utilities|Array|Get(acopy) _returnvalue _returnvalue_4))
  (bind _returnvalue_5 (Transformation|GetActorTransform _item))
  (Utilities|IsValid PlayerController
    (:Is%20Valid
      (bind _returnvalue_6 (Game|SpawnActorfromClass "/Game/MP_FPS/Blueprints/Characters/BP_CharacterMaster.BP_CharacterMaster_C" (Math|Transform|MakeTransform (.location _returnvalue_5) (.rotation _returnvalue_5) "1,1,1") "AdjustIfPossibleButAlwaysSpawn" 0 team 0))
      (Utilities|IsValid _returnvalue_6
        (:Is%20Valid
          (Pawn|Possess PlayerController _returnvalue_6))))))

(event EventBeginPlay
  (Utilities|FlowControl|Delay 0.5)
  (Networking|SwitchHasAuthority
    (:Authority
      (bind _outactors (Actor|GetAllActorsOfClass "/Game/MP_FPS/Blueprints/PlayerStart/BP_TeamStartMaster.BP_TeamStartMaster_C"))
      (for _array_element _outactors
        (if (Utilities|Enum|Equal(Enum) (Variables|/Game/MP_FPS/Blueprints/PlayerStart/BP_TeamStartMaster.BP_TeamStartMaster_C|Getteam _array_element) "NewEnumerator0")
          (Utilities|Array|Add (Variables|Default|GetlobbySpawnPoints) _array_element)
          (elif (Utilities|Enum|Equal(Enum) (Variables|/Game/MP_FPS/Blueprints/PlayerStart/BP_TeamStartMaster.BP_TeamStartMaster_C|Getteam _array_element) "NewEnumerator1")
            (Utilities|Array|Add (Variables|Default|GetredTeamSpawnPoints) _array_element)
            (elif (Utilities|Enum|Equal(Enum) (Variables|/Game/MP_FPS/Blueprints/PlayerStart/BP_TeamStartMaster.BP_TeamStartMaster_C|Getteam _array_element) "NewEnumerator2")
              (Utilities|Array|Add (Variables|Default|GetblueTeamSpawnPoints) _array_element))))))))

(fn ConstructionScript)