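; Master weapon for a multiplayer FPS, handling firing in hitscan or projectile mode with separate first- and third-person meshes.
; The client sphere-traces from the camera to find the aim point, then from the muzzle toward it, and sends that hit to the server.
; The server applies damage or spawns a projectile, then multicasts sound, per-view muzzle flashes and hitscan impacts.
; The first-person projectile call sits behind a disabled branch.
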(event Custom|ClientOnWeaponFire
  (bind _bp_charactermasterreference (Variables|Default|GetBP_CharacterMasterReference))
  (bind _array (Utilities|Array|MakeArray _bp_charactermasterreference))
  (bind _fp_camera (Variables|/Game/MP_FPS/Blueprints/Characters/BP_CharacterMaster.BP_CharacterMaster_C|GetFP_Camera _bp_charactermasterreference))
  (bind _returnvalue (Transformation|GetWorldLocation _fp_camera))
  (bind (_outhit _returnvalue_2) (Collision|SphereTraceByChannel _returnvalue (+ _returnvalue (* (Math|Vector|GetForwardVector _fp_camera) (Variables|Default|GetweaponRange))) (Variables|Default|GetshotRadius) "TraceTypeQuery1" false _array "None"))
  (bind (_outhit_2 _returnvalue_3) (Collision|SphereTraceByChannel (Transformation|GetSocketLocation (Variables|Default|GetSK_FP_Weapon) (Variables|Default|GetmuzzleSocketName)) (Math|Vector|SelectVector (.ImpactPoint (Collision|BreakHitResult _outhit)) (.TraceEnd (Collision|BreakHitResult _outhit)) _returnvalue_2) (Variables|Default|GetshotRadius) "TraceTypeQuery1" false _array "None"))
  (if true
    _
    (else
      (CallFunction|ClientShootInfo)))
  (CallFunction|ServerShootInfo _outhit_2 _returnvalue_3))

(event Custom|ClientShootInfo
  (params (HitResult :type Hit%20Result%20Structure) (hit :type Boolean))
  (bind (_bblockinghit _binitialoverlap _time _location _impactpoint _normal _impactnormal _physmat _hitactor _hitcomponent _hitbonename _hititem _faceindex _tracestart _traceend) (Collision|BreakHitResult HitResult))
  (if (not (Variables|Default|GetisHitscan))
    (Game|SpawnActorfromClass "/Game/MP_FPS/Blueprints/Weapons/BP_FP_ProjectileMaster.BP_FP_ProjectileMaster_C" (Math|Transform|MakeTransform "0, 0, 0" (Math|Rotator|FindLookatRotation (Transformation|GetSocketLocation (Variables|Default|GetSK_FP_Weapon) (Variables|Default|GetmuzzleSocketName)) (Math|Vector|SelectVector _impactpoint _traceend hit))) "AlwaysSpawn" (Components|GetOwner) (Game|GetInstigator))))

(event Custom|MulticastWeaponFX
  (params (HitResult :type Hit%20Result%20Structure) (didHit :type Boolean))
  (bind (_bblockinghit _binitialoverlap _time _location _impactpoint _normal _impactnormal) (Collision|BreakHitResult HitResult))
  (bind _sk_fp_weapon (Variables|Default|GetSK_FP_Weapon))
  (Audio|SpawnSoundAttached (Variables|Default|GetfireWeaponSound) _sk_fp_weapon "MuzzleFlash")
  (Utilities|FlowControl|Sequence
    (:then_0
      ;[1 1 1] First Person muzzle flash emitter
      (bind _returnvalue (Effects|SpawnEmitterAttached (Variables|Default|GetPS_muzzleFlash) _sk_fp_weapon (Variables|Default|GetmuzzleSocketName) "0, 0, 0" "0, 0, 0" "SnapToTarget"))
      (Rendering|SetOnlyOwnerSee _returnvalue true :!class /Script/Engine.PrimitiveComponent)
      (if (Variables|Default|GetisHitscan)
        (if didHit
          (Audio|PlaySoundatLocation (Variables|Default|GetimpactSound) _impactpoint)
          (Effects|SpawnEmitteratLocation (Variables|Default|GetPS_Impact) _impactpoint (Math|Rotator|MakeRotfromZ _impactnormal)))))
    (:then_1
      ;[1 1 1] Third person muzzle flash emitter
      (bind _returnvalue_2 (Effects|SpawnEmitterAttached (Variables|Default|GetPS_muzzleFlash) (Variables|Default|GetSK_TP_Weapon) (Variables|Default|GetmuzzleSocketName) "0, 0, 0" "0, 0, 0" "SnapToTarget"))
      (Class|PrimitiveComponent|SetOwnerNoSee _returnvalue_2 true))))

(event Custom|ClientOffWeaponFire)

(event Custom|ServerShootInfo
  (params (HitResult :type Hit%20Result%20Structure) (didHit :type Boolean))
  (bind (_bblockinghit _binitialoverlap _time _location _impactpoint _normal _impactnormal _physmat _hitactor _hitcomponent _hitbonename _hititem _faceindex _tracestart _traceend) (Collision|BreakHitResult HitResult))
  (bind _muzzlesocketname (Variables|Default|GetmuzzleSocketName))
  (bind _sk_tp_weapon (Variables|Default|GetSK_TP_Weapon))
  (bind _returnvalue (Transformation|GetSocketLocation _sk_tp_weapon _muzzlesocketname))
  (if (Variables|Default|GetisHitscan)
    (Game|Damage|ApplyDamage _hitactor (Math|Conversions|ToFloat(Integer) (Variables|Default|Getdamage)) (Game|GetInstigatorController) self)
    (else
      (Game|SpawnActorfromClass "/Game/MP_FPS/Blueprints/Weapons/BP_TP_ProjectileMaster.BP_TP_ProjectileMaster_C" (Math|Transform|MakeTransform _returnvalue (Math|Rotator|FindLookatRotation _returnvalue (Math|Vector|SelectVector _impactpoint _traceend didHit))) "AlwaysSpawn" (Components|GetOwner) (Game|GetInstigator))))
  (CallFunction|MulticastWeaponFX HitResult didHit))

(fn ConstructionScript)